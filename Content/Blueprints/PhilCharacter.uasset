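; PhilCharacter is a player character Blueprint with camera-relative movement, mouse look, double jump and wall climbing.
; Each Tick, a trace toward LineEndLocation finds "Climable" actors; holding Space there repeatedly launches the character upward for a short time window.
; That hold time, stored in ClimbTime, blocks movement input while nonzero.
; A DoN gate makes the second jump a launch, resets on landing and prints its count.
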(event `self.ReceiveTick`
  (params (DeltaSeconds :type "Float (single-precision)"))
  ;[1 1 1] Climbing
  (bind _outhit (`KismetSystemLibrary.LineTraceSingle` :`Start` (`self.K2_GetActorLocation`) :`End` (`SceneComponent.K2_GetComponentLocation` (`self.LineEndLocation`)) :`TraceChannel` "TraceTypeQuery1" :`DrawDebugType` "ForDuration"))
  (if (`self.ActorHasTag` (`.HitActor` (`GameplayStatics.BreakHitResult` _outhit)) "Climable")
    (bind _output_get (set `self.ClimbTime` (`PlayerController.GetInputKeyTimeDown` (`GameplayStatics.GetPlayerController` 0) "SpaceBar")))
    (if (!= _output_get 0.0)
      (if (<= _output_get 0.7)
        (`self.LaunchCharacter` (0.0 0.0 500.0) true true)))
    (else
      (set `self.ClimbTime` 0.0))))

(event `InputAxis|MoveHorizontal`
  (params (AxisValue :type "Float (single-precision)"))
  (bind (_returnvalue_roll _returnvalue_pitch _returnvalue_yaw) (`KismetMathLibrary.BreakRotator` (`self.GetControlRotation`)))
  ;[1 1 1] Movement
  (if (== (`self.ClimbTime`) 0.0)
    (`self.AddMovementInput` (`KismetMathLibrary.GetRightVector` (`KismetMathLibrary.MakeRotator` 0.0 0.0 _returnvalue_yaw)) AxisValue)))

(event `InputAxis|MoveVertical`
  (params (AxisValue :type "Float (single-precision)"))
  (bind (_returnvalue_roll _returnvalue_pitch _returnvalue_yaw) (`KismetMathLibrary.BreakRotator` (`self.GetControlRotation`)))
  ;[1 1 1] Movement
  (if (== (`self.ClimbTime`) 0.0)
    (`self.AddMovementInput` (`KismetMathLibrary.GetForwardVector` (`KismetMathLibrary.MakeRotator` 0.0 0.0 _returnvalue_yaw)) AxisValue)))

(event `InputAxis|MouseLookHorizontal`
  (params (AxisValue :type "Float (single-precision)"))
  ;[1 1 1] Camera
  (`self.AddControllerYawInput` AxisValue))

(event `InputAction|Jump`
  (params (Key :type "Key Structure"))
  ;[1 1 1] DoubleJump
  (:`Pressed`
    (bind _counter (`/Engine/EditorBlueprintResources/StandardMacros.Do N` 2 :!label _label)
      (:`Exit`
        (`KismetSystemLibrary.PrintString` (`KismetStringLibrary.Conv_IntToString` _counter))
        (switch `int` _counter
          (:`1`
            (`self.Jump`))
          (:`2`
            (`self.LaunchCharacter` (0.0 0.0 500.0))))))))

(event `self.OnLanded`
  (params (Hit :type "HitResult Structure (by ref)"))
  ;[1 1 1] DoubleJump
  (goto _label :!via `Reset`))

(event `InputAxis|MouseLookVertical`
  (params (AxisValue :type "Float (single-precision)"))
  ;[1 1 1] Camera
  (`self.AddControllerPitchInput` AxisValue))

(fn `UserConstructionScript`)