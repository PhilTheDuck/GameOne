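; Button_BP is a pressable button actor that responds to the Interact input while a PhilCharacter overlaps its Box trigger.
; Box overlaps open and close a gate on the input, which plays a sound call at world origin and starts the Button_in timeline.
; That timeline lerps the Button inward along local X, then reverses Timeline_0, whose transform update is unconnected.
; The press triggers nothing else.
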(event `self.ReceiveBeginPlay`
  (bind (_returnvalue_location _returnvalue_rotation _returnvalue_scale) (`KismetMathLibrary.BreakTransform` (`SceneComponent.GetRelativeTransform` (`self.Button`))))
  (set `self.OutPosition` (`KismetMathLibrary.MakeTransform` _returnvalue_location _returnvalue_rotation _returnvalue_scale))
  (set `self.InPosition` (`KismetMathLibrary.MakeTransform` (- _returnvalue_location (10.0 0.0 0.0)) _returnvalue_rotation _returnvalue_scale))
  (`self.EnableInput` (`GameplayStatics.GetPlayerController` 0)))

(event `InputAction|Interact`
  (params (Key :type "Key Structure"))
  (:`Pressed`
    (`/Engine/EditorBlueprintResources/StandardMacros.Gate` true :!label _label
      (:`Exit`
        (`GameplayStatics.PlaySoundAtLocation` null (0.0 0.0 0.0) (struct) 1.0 1.0 0.0 null null null)
        (bind (_direction _button_in) (`Timeline|Button_in` :!via `PlayFromStart`)
          (:`Update`
            (`SceneComponent.K2_SetRelativeTransform` (`self.Button`) (`KismetMathLibrary.TLerp` (`self.OutPosition`) (`self.InPosition`) _button_in) false false))
          (:`Finished`
            (bind (_direction_2 _button_in_2) (`Timeline|Timeline_0` :!via `ReverseFromEnd`))))))))

(event `self.Box.OnComponentBeginOverlap`
  (params (OverlappedComponent :type "PrimitiveComponent Object Reference") (OtherActor :type "Actor Object Reference") (OtherComp :type "PrimitiveComponent Object Reference") (OtherBodyIndex :type Integer) (bFromSweep :type Boolean) (SweepResult :type "HitResult Structure (by ref)"))
  (cast `/Game/Blueprints/PhilCharacter` OtherActor)
  (goto _label :!via `Open`))

(event `self.Box.OnComponentEndOverlap`
  (params (OverlappedComponent :type "PrimitiveComponent Object Reference") (OtherActor :type "Actor Object Reference") (OtherComp :type "PrimitiveComponent Object Reference") (OtherBodyIndex :type Integer))
  (cast `/Game/Blueprints/PhilCharacter` OtherActor)
  (goto _label :!via `Close`))

(fn `UserConstructionScript`)